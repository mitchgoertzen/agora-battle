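; Master character for a grid-placement battle game, holding stats, a derived cost and a toggleable percentage bonus to attack and defence.
; Hovering shows stats in the owning grid's menu and, for placed characters, sets the active character.
; Outside battle, dragging follows a mouse-ray projection onto the ground; release snaps to the overlapped active block or returns to the last position.
; During battle, Tick cycles a four-montage attack combo.
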(event OnClicked(Box)
  (params (TouchedComponent :type Primitive%20Component%20Object%20Reference) (ButtonPressed :type Key%20Structure :default "None"))
  ;[1 1 1] Handle Mouse Click
  (Variables|Default|Setmouse%20held true))

(event OnReleased(Box)
  (params (TouchedComponent :type Primitive%20Component%20Object%20Reference) (ButtonReleased :type Key%20Structure :default "None"))
  ;[1 1 1] Handle Mouse Click
  (Variables|Default|Setmouse%20held false)
  (if (Utilities|IsValid (Variables|/Game/Blueprints/PuzzleBlockGrid.PuzzleBlockGrid_C|GetActive%20Block (Variables|Default|Getowning%20gird)))
    (if (Class|PrimitiveComponent|IsOverlappingComponent (Variables|Default|GetBox) (Variables|/Game/Blueprints/PuzzleBlock.PuzzleBlock_C|GetBox (Variables|/Game/Blueprints/PuzzleBlockGrid.PuzzleBlockGrid_C|GetActive%20Block (Variables|Default|Getowning%20gird))))
      (bind _output_get (Variables|Default|Setnext%20block (Variables|/Game/Blueprints/PuzzleBlockGrid.PuzzleBlockGrid_C|GetActive%20Block (Variables|Default|Getowning%20gird))))
      (if (Utilities|IsValid (Variables|Default|Getcurrent%20block))
        (if (== _output_get (Variables|Default|Getcurrent%20block))
          _
          (else
            (Default|RemoveCharacter (Variables|Default|Getcurrent%20block))
            (bind _output_get_2 (Variables|Default|Setstarting%20location (Math|Vector|MakeVector (.X (Math|Vector|BreakVector (Transformation|GetActorLocation (Variables|/Game/Blueprints/PuzzleBlockGrid.PuzzleBlockGrid_C|GetActive%20Block (Variables|Default|Getowning%20gird))))) (.Y (Math|Vector|BreakVector (Transformation|GetActorLocation (Variables|/Game/Blueprints/PuzzleBlockGrid.PuzzleBlockGrid_C|GetActive%20Block (Variables|Default|Getowning%20gird))))) (+ (.Z (Math|Vector|BreakVector (Transformation|GetActorLocation (Variables|/Game/Blueprints/PuzzleBlockGrid.PuzzleBlockGrid_C|GetActive%20Block (Variables|Default|Getowning%20gird))))) 5e+01)) :!label _label))
            (if (Variables|Default|GetinPlay)
              _
              (else
                (Default|PlaceCharacteronGrid (Variables|Default|Getowning%20gird) self)))
            (Default|PlaceCharacter (Variables|Default|Getnext%20block) self)
            (Variables|Default|Setcurrent%20block (Variables|Default|Getnext%20block))))
        (else
          (goto _label)))
      (Transformation|SetActorRelativeLocation _output_get_2)
      (Variables|/Game/Blueprints/PuzzleBlockGrid.PuzzleBlockGrid_C|SetActive%20Block (Variables|Default|Getowning%20gird) 0)
      (else
        (Transformation|SetActorRelativeLocation (Variables|Default|Getstarting%20location) :!label _label_2)
        (Variables|/Game/Blueprints/PuzzleBlockGrid.PuzzleBlockGrid_C|SetActive%20Block (Variables|Default|Getowning%20gird) 0)))
    (else
      (goto _label_2))))

(event Custom|Reset%20Combo
  ;[1 1 1] Fighting
  (Variables|Default|SetattackCount 0)
  (Variables|Default|SetisAttacking false))

(event MouseInput|EventActorBeginCursorOver
  ;[1 1 1] Handle Mouse Over
  (bind (_name _attack _defence _class) (CallFunction|GetInfo))
  (Default|SetInfo (Variables|/Game/Blueprints/PuzzleBlockGrid.PuzzleBlockGrid_C|Getmenu (Variables|Default|Getowning%20gird)) 0 _name _attack _defence _class)
  (if (Variables|Default|GetinPlay)
    (Default|Setactivechacrter (Variables|Default|Getowning%20gird) true self)))

(event MouseInput|EventActorEndCursorOver
  ;[1 1 1] Handle Mouse Over
  (Default|ClearInfo (Variables|/Game/Blueprints/PuzzleBlockGrid.PuzzleBlockGrid_C|Getmenu (Variables|Default|Getowning%20gird)))
  (if (Variables|Default|GetinPlay)
    (Default|Setactivechacrter (Variables|Default|Getowning%20gird) false)))

(event EventTick
  (params (DeltaSeconds :type Float%20%28single-precision%29))
  (bind _returnvalue (Game|GetPlayerController 0))
  (bind (_worldlocation _worlddirection) (Game|Player|ConvertMouseLocationToWorldSpace _returnvalue))
  (bind _z (Math|Vector|BreakVector _worldlocation))
  (bind _z_2 (Math|Vector|BreakVector _worlddirection))
  (bind _returnvalue_2 (/ _z _z_2))
  (bind _returnvalue_3 (* _worlddirection _returnvalue_2))
  (bind _returnvalue_4 (* _returnvalue_3 -1.0))
  (bind _returnvalue_5 (+ _worldlocation _returnvalue_4))
  (bind (_x _y _z_3) (Math|Vector|BreakVector _returnvalue_5))
  ;[1 1 1] Tick
  (if (Variables|Default|GetisBattlePhase)
    ;[1 1 1] Fighting
    (if (not (Variables|Default|GetisAttacking))
      (Variables|Default|SetisAttacking true)
      (switch int (Variables|Default|GetattackCount)
        (:0
          (Variables|Default|SetattackCount 1)
          (bind _returnvalue_6 (Animation|PlayAnimMontage (Variables|Default|Getattack_0) 1.0 "None"))
          (Utilities|FlowControl|Delay _returnvalue_6)
          (Variables|Default|SetisAttacking false))
        (:1
          (Variables|Default|SetattackCount 2)
          (bind _returnvalue_7 (Animation|PlayAnimMontage (Variables|Default|Getattack_1) 1.0 "None"))
          (Utilities|FlowControl|Delay _returnvalue_7)
          (Variables|Default|SetisAttacking false))
        (:2
          (Variables|Default|SetattackCount 3)
          (bind _returnvalue_8 (Animation|PlayAnimMontage (Variables|Default|Getattack_2) 1.0 "None"))
          (Utilities|FlowControl|Delay _returnvalue_8)
          (Variables|Default|SetisAttacking false))
        (:3
          (Variables|Default|SetattackCount 0)
          (bind _returnvalue_9 (Animation|PlayAnimMontage (Variables|Default|Getattack_3) 1.0 "None"))
          (Utilities|FlowControl|Delay _returnvalue_9)
          (Variables|Default|SetisAttacking false)
          (CallFunction|ResetCombo))))
    (elif (Variables|Default|Getmouse%20held)
      ;[1 1 1] Get Location from Mouse
      (Transformation|SetActorRelativeLocation (Math|Vector|MakeVector _x _y (+ _z_3 5e+01))))))

(event EventBeginPlay
  ;[1 1 1] Initialize Attributes
  (Variables|Default|SetCost (/ (* (Variables|Default|GetAttack) (Variables|Default|GetDefence)) 100))
  (Variables|Default|Setstarting%20location (Transformation|GetActorLocation)))

(fn ConstructionScript)

(fn GetAttack
  (return (Variables|Default|GetAttack)))

(fn GetDefence
  (return (Variables|Default|GetDefence)))

(fn GetClass
  (return (Variables|Default|GetClass)))

(fn AddBonus
  (if (not (Variables|Default|GetbonusActive))
    (Variables|Default|SetAttack (+ (Variables|Default|GetAttack) (Math|Float|Truncate (* (Variables|Default|GetAttack) 0.1))))
    (Variables|Default|SetDefence (+ (Variables|Default|GetDefence) (Math|Float|Truncate (* (Variables|Default|GetDefence) 0.1))))
    (Variables|Default|SetbonusActive true)))

(fn RemoveBonus
  (if (Variables|Default|GetbonusActive)
    (Variables|Default|SetAttack (- (Variables|Default|GetAttack) (Math|Float|Truncate (* (Variables|Default|GetAttack) 0.1))))
    (Variables|Default|SetDefence (- (Variables|Default|GetDefence) (Math|Float|Truncate (* (Variables|Default|GetDefence) 0.1))))
    (Variables|Default|SetbonusActive false)))

(fn GetCost
  (return (Variables|Default|GetCost)))

(fn GetStoreAmount
  (return (Variables|Default|GetStore%20Amount)))

(fn ResetCombo)

(fn GetInfo
  (return (Variables|Default|GetName) (Variables|Default|GetAttack) (Variables|Default|GetDefence) (Variables|Default|GetClass)))

(fn GetName
  (return (Variables|Default|GetName)))