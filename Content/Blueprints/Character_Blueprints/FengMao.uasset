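; FengMao is a character Blueprint that the player can pick up and drag with the mouse by clicking its Box component.
; While the mouse is held, Tick intersects the deprojected cursor ray with the world Z=0 plane and moves the actor above that point.
; On release, it clears the grab state and lowers the actor by a fixed offset, without sweeping for collision.
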(event OnClicked(Box)
  (params (TouchedComponent :type Primitive%20Component%20Object%20Reference) (ButtonPressed :type Key%20Structure :default "None"))
  (Variables|Default|Setmouse%20held true))

(event OnReleased(Box)
  (params (TouchedComponent :type Primitive%20Component%20Object%20Reference) (ButtonReleased :type Key%20Structure :default "None"))
  (bind _returnvalue (Transformation|GetActorLocation))
  (bind (_x _y _z) (Math|Vector|BreakVector _returnvalue))
  (Variables|Default|Setmouse%20held false)
  (if (Variables|Default|Getgrabbing)
    (Variables|Default|Setgrabbing false)
    (Transformation|SetActorRelativeLocation (Math|Vector|MakeVector _x _y (+ _z -5e+01)))))

(event EventTick
  (params (DeltaSeconds :type Float%20%28single-precision%29))
  (bind _returnvalue (Game|GetPlayerController 0))
  (bind (_worldlocation _worlddirection) (Game|Player|ConvertMouseLocationToWorldSpace _returnvalue))
  (bind _z (Math|Vector|BreakVector _worldlocation))
  (bind _z_2 (Math|Vector|BreakVector _worlddirection))
  (bind _returnvalue_2 (/ _z _z_2))
  (bind _returnvalue_3 (* _worlddirection _returnvalue_2))
  (bind _returnvalue_4 (* _returnvalue_3 -1.0))
  (bind _returnvalue_5 (+ _worldlocation _returnvalue_4))
  (bind (_x _y _z_3) (Math|Vector|BreakVector _returnvalue_5))
  (if (Variables|Default|Getmouse%20held)
    (Variables|Default|Setgrabbing true)
    (Transformation|SetActorRelativeLocation (Math|Vector|MakeVector _x _y (+ _z_3 1e+02)))))

(fn ConstructionScript)