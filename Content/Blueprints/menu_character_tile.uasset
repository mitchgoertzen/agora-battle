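; A clickable 3D tile that represents one character in a menu and spawns that character on the menu's grid.
; Cursor hover over the static mesh marks the tile active and sets its character as the menu's selection, and leaving clears both.
; A click while active asks the owning menu's grid to spawn the tile's character.
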(event OnClicked(StaticMeshComponent)
  (params (TouchedComponent :type Primitive%20Component%20Object%20Reference) (ButtonPressed :type Key%20Structure :default "None"))
  (if (Variables|Default|GetisActive)
    (Default|SpawnCharacter (Variables|/Game/Blueprints/menu.menu_C|Getowning%20grid (Variables|Default|Getowning%20menu)) (Variables|Default|Getowning_character))))

(event OnBeginCursorOver(StaticMeshComponent)
  (params (TouchedComponent :type Primitive%20Component%20Object%20Reference))
  (Variables|Default|SetisActive true)
  (Variables|/Game/Blueprints/menu.menu_C|Setselected%20character (Variables|Default|Getowning%20menu) (Variables|Default|Getowning_character)))

(event OnEndCursorOver(StaticMeshComponent)
  (params (TouchedComponent :type Primitive%20Component%20Object%20Reference))
  (Variables|Default|SetisActive false)
  (Variables|/Game/Blueprints/menu.menu_C|Setselected%20character (Variables|Default|Getowning%20menu) 0))

(fn ConstructionScript)