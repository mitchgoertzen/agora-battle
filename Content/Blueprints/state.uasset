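; Game state actor that alternates planning and battle phases, showing the phase on a text render.
; Tick updates a per-second planning countdown, while a latent Delay of PlanningTime triggers the Ai actor's MakeDecision and starts battle.
; EndBattlePhase adds funds to every PuzzleBlockGrid menu, reinitializes it and resumes planning.
; EndGame sets GameOver and displays the message, though Tick never checks that flag.
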(event EventTick
  (params (DeltaSeconds :type Float%20%28single-precision%29))
  (if (Variables|Default|Getbattle%20phase)
    (Variables|Default|Settime 0.0)
    (Variables|Default|Setcheck 0.0)
    (Variables|Default|Setprint%20time (Variables|Default|Getplanning%20time))
    (else
      (bind _output_get (Variables|Default|Settime (+ (Variables|Default|Gettime) DeltaSeconds)))
      (if (> _output_get (Variables|Default|Getcheck))
        (Variables|Default|Setcheck (+ (Variables|Default|Getcheck) 1.0))
        (bind _output_get_2 (Variables|Default|Setprint%20time (- (Variables|Default|Getplanning%20time) (Math|Float|Truncate _output_get))))
        (Rendering|Components|TextRender|SetText (Variables|Default|GetTextRender) (Utilities|Text|FormatText "Planning: {Time}" _output_get_2))
        (Utilities|FlowControl|Delay (Math|Conversions|ToFloat(Integer) (Variables|Default|Getplanning%20time)))
        (bind _returnvalue (Actor|GetActorOfClass "/Game/Blueprints/ai.ai_C"))
        (Default|MakeDecision _returnvalue)
        (Variables|Default|Setbattle%20phase true)
        (Rendering|Components|TextRender|SetText (Variables|Default|GetTextRender) (Utilities|Text|FormatText "Battle"))
        (Utilities|FlowControl|Delay 3.0)))))

(event Collision|EventActorBeginOverlap
  (params (OtherActor :type Actor%20Object%20Reference)))

(event EventBeginPlay)

(fn ConstructionScript)

(fn EndBattlePhase
  (bind _outactors (Actor|GetAllActorsOfClass "/Game/Blueprints/PuzzleBlockGrid.PuzzleBlockGrid_C"))
  (for _array_element _outactors
    (Variables|/Game/Blueprints/menu.menu_C|SetAvailable%20Funds (Variables|/Game/Blueprints/PuzzleBlockGrid.PuzzleBlockGrid_C|Getmenu _array_element) (+ (Variables|/Game/Blueprints/menu.menu_C|GetAvailable%20Funds (Variables|/Game/Blueprints/PuzzleBlockGrid.PuzzleBlockGrid_C|Getmenu _array_element)) 2500))
    (Default|InitMenu (Variables|/Game/Blueprints/PuzzleBlockGrid.PuzzleBlockGrid_C|Getmenu _array_element)))
  (Variables|Default|Setbattle%20phase false))

(fn EndGame
  (Variables|Default|Setgame%20over true)
  (Rendering|Components|TextRender|SetText (Variables|Default|GetTextRender) (Utilities|Text|FormatText "GAME OVER")))