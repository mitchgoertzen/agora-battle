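; Character shop menu actor that offers five random picks from a rarity-weighted pool of hero classes and tracks available funds.
; InitMenu rebuilds the offer and, for human-owned grids only, spawns a row of tiles with dynamic-material portraits.
; Tile stats come from briefly spawning each character below the world origin, reading its getters, then destroying it.
; Info functions show stats and preview remaining funds, while purchasing deducts cost and removes the character from the master pool.
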(event Custom|init%20menu
  (bind _available_characters (Variables|Default|Getavailable_characters))
  (Variables|Default|Setcharacter%20pool (Variables|Default|Getall%20chars))
  (if (Variables|/Game/Blueprints/PuzzleBlockGrid.PuzzleBlockGrid_C|Gethuman (Variables|Default|Getowning%20grid))
    (Rendering|Components|TextRender|SetText (Variables|Default|Getfunds) (Utilities|Text|FormatText "Available Funds: {Available Funds}" (Variables|Default|GetAvailable%20Funds)))
    (else
      (Rendering|Components|TextRender|SetText (Variables|Default|Getfunds) (Utilities|Text|FormatText ""))))
  (for _array_element (Variables|Default|Gettiles)
    (if (Utilities|IsValid _array_element)
      (Actor|DestroyActor _array_element)))
  (Utilities|Array|Clear (Variables|Default|Gettiles))
  (Utilities|Array|Clear (Variables|Default|Getavailable_characters))
  (for _index (range 0 4)
    (Utilities|Array|Add _available_characters (Utilities|Array|Get(acopy) (Variables|Default|Getcharacter%20pool) (Math|Random|RandomInteger (- (Utilities|Array|Length (Variables|Default|Getcharacter%20pool)) 1))))
    (Utilities|Array|RemoveIndex (Variables|Default|Getcharacter%20pool) (Math|Random|RandomInteger (- (Utilities|Array|Length (Variables|Default|Getcharacter%20pool)) 1))))
  (if (Variables|/Game/Blueprints/PuzzleBlockGrid.PuzzleBlockGrid_C|Gethuman (Variables|Default|Getowning%20grid))
    (for _array_element_2 _available_characters
      (bind _tile (CallFunction|SpawnTile _array_element_2))
      (Utilities|Array|Add (Variables|Default|Gettiles) _tile))))

(event EventBeginPlay
  (bind _character_pool (Variables|Default|Getcharacter%20pool))
  (Variables|Default|SetAvailable%20Funds 3000)
  (Utilities|FlowControl|Sequence
    (:then_0
      (for _index (range 0 9)
        (Utilities|Array|Add _character_pool "/Game/Blueprints/Character_Blueprints/Crunch.Crunch_C")))
    (:then_1
      (for _index_2 (range 0 4)
        (Utilities|Array|Add _character_pool "/Game/Blueprints/Character_Blueprints/FengMao.FengMao_C")))
    (:then_2
      (for _index_3 (range 0 19)
        (Utilities|Array|Add _character_pool "/Game/Blueprints/Character_Blueprints/Gideon.Gideon_C")))
    (:then_3
      (for _index_4 (range 0 9)
        (Utilities|Array|Add _character_pool "/Game/Blueprints/Character_Blueprints/Kallari.Kallari_C")))
    (:then_4
      (for _index_5 (range 0 4)
        (Utilities|Array|Add _character_pool "/Game/Blueprints/Character_Blueprints/Khaimera.Khaimera_C")))
    (:then_5
      (for _index_6 (range 0 14)
        (Utilities|Array|Add _character_pool "/Game/Blueprints/Character_Blueprints/Rampage.Rampage_C")))
    (:then_6
      (for _index_7 (range 0 9)
        (Utilities|Array|Add _character_pool "/Game/Blueprints/Character_Blueprints/Steel.Steel_C")))
    (:then_7
      (Variables|Default|Setall%20chars (Variables|Default|Getcharacter%20pool))
      (CallFunction|InitMenu))))

(fn ConstructionScript)

(fn SpawnTile
  (params (owning%20character :type Game%20Character%20Master%20Class%20Reference))
  (bind _returnvalue (Transformation|GetActorLocation))
  (bind (_x _y _z) (Math|Vector|BreakVector _returnvalue))
  (bind (_cost _attack _defence _class_type _name) (CallFunction|GetCharacterAttributes owning%20character))
  (bind _returnvalue_2 (Game|SpawnActorfromClass "/Game/Blueprints/menu_character_tile.menu_character_tile_C" (Math|Transform|MakeTransform (Math|Vector|MakeVector (+ (* (Utilities|Array|Length (Variables|Default|Gettiles)) 1.5e+02) _x) _y _z) (Math|Rotator|MakeRotator 35.0 0.0 0.0)) "Undefined" 0 _cost _attack _defence _class_type _name 0))
  (switch string (Utilities|GetClassDisplayName owning%20character)
    (:crunch_c
      (Variables|Default|Settexture "/Game/Images/crunch_preview.crunch_preview"))
    (:fengmao_c
      (Variables|Default|Settexture "/Game/Images/feng_preview.feng_preview"))
    (:gideon_c
      (Variables|Default|Settexture "/Game/Images/gideon_preview.gideon_preview"))
    (:kallari_c
      (Variables|Default|Settexture "/Game/Images/kallari_preview.kallari_preview"))
    (:khaimera_c
      (Variables|Default|Settexture "/Game/Images/khaimera_preview.khaimera_preview"))
    (:rampage_c
      (Variables|Default|Settexture "/Game/Images/rampage_preview.rampage_preview"))
    (:steel_c
      (Variables|Default|Settexture "/Game/Images/steel_preview.steel_preview")))
  (Variables|/Game/Blueprints/menu_character_tile.menu_character_tile_C|Setowning_character _returnvalue_2 owning%20character)
  (Variables|/Game/Blueprints/menu_character_tile.menu_character_tile_C|Setowning%20menu _returnvalue_2 self)
  (bind _returnvalue_3 (Rendering|Material|CreateDynamicMaterialInstance "/Game/Materials/character_preview.character_preview" "None" "None" :!class /Script/Engine.KismetMaterialLibrary))
  (Variables|Default|Setmaterial _returnvalue_3)
  (Rendering|Material|SetTextureParameterValue (Variables|Default|Getmaterial) "Param" (Variables|Default|Gettexture))
  (Rendering|Material|SetMaterial (Variables|/Script/Engine.StaticMeshActor|GetStaticMeshComponent _returnvalue_2) 0 (Variables|Default|Getmaterial))
  (return _returnvalue_2))

(fn PurchaseCharacter
  (params (cost :type Integer) (char :type Game%20Character%20Master%20Class%20Reference))
  (Utilities|Array|RemoveItem (Variables|Default|Getall%20chars) char)
  (bind _output_get (Variables|Default|SetAvailable%20Funds (- (Variables|Default|GetAvailable%20Funds) cost)))
  (Rendering|Components|TextRender|SetText (Variables|Default|Getfunds) (Utilities|Text|FormatText "Available Funds {Available Funds}" _output_get))
  (CallFunction|ClearInfo))

(fn GetCharacterAttributes
  (params (character :type Game%20Character%20Master%20Class%20Reference))
  (bind _returnvalue (Game|SpawnActorfromClass character (Math|Transform|MakeTransform "0, 0,-1000.000000") "Undefined" 0 0 0))
  (Utilities|FlowControl|Sequence
    (:then_0
      (bind _cost (Default|GetCost _returnvalue)))
    (:then_1
      (bind _attack (Default|GetAttack _returnvalue)))
    (:then_2
      (bind _defence (Default|GetDefence _returnvalue)))
    (:then_3
      (bind _class (Default|GetClass _returnvalue)))
    (:then_4
      (bind _name (Default|GetName _returnvalue)))
    (:then_5
      (Actor|DestroyActor _returnvalue)
      (return _cost _attack _defence _class _name))))

(fn SetInfo
  (params (cost :type Integer) (name :type String) (attack :type Integer) (defence :type Integer) (class :type String))
  (bind _funds (Variables|Default|Getfunds))
  (bind _available_funds (Variables|Default|GetAvailable%20Funds))
  (bind _returnvalue (- _available_funds cost))
  (Variables|Default|Setcost "")
  (bind _output_get (Variables|Default|Setcost%20not%20zero (> cost 0)))
  (if _output_get
    (bind _output_get_2 (Variables|Default|Setcost (Utilities|String|Append (Utilities|String|Append "Cost: " (Utilities|String|ToString(Integer) cost)) ""))))
  (Rendering|Components|TextRender|SetText (Variables|Default|GetCharacter%20Info) (Utilities|Text|FormatText (Utilities|Text|ToText(String) (Utilities|String|Append (Utilities|String|Append (Utilities|String|Append (Utilities|String|Append (Utilities|String|Append (Utilities|String|Append (Utilities|String|Append (Utilities|String|Append _output_get_2 " 
Name: ") name) " 
Attack: ") (Utilities|String|ToString(Integer) attack)) " 
Defence: ") (Utilities|String|ToString(Integer) defence)) " 
Class: ") class))))
  (if (Variables|/Game/Blueprints/PuzzleBlockGrid.PuzzleBlockGrid_C|Gethuman (Variables|Default|Getowning%20grid))
    (Rendering|Components|TextRender|SetText _funds (Utilities|Text|FormatText "Available Funds: {Available Funds}" _returnvalue))
    (if (Variables|Default|Getcost%20not%20zero)
      (if (> _returnvalue 0)
        (Rendering|Components|TextRender|SetTextRenderColor _funds (Math|Color|MakeColor 110 110 255 100))
        (else
          (Rendering|Components|TextRender|SetTextRenderColor _funds (Math|Color|MakeColor 0 0 150 100)))))
    (else
      (Rendering|Components|TextRender|SetText (Variables|Default|Getfunds) (Utilities|Text|FormatText "")))))

(fn ClearInfo
  (bind _funds (Variables|Default|Getfunds))
  (Rendering|Components|TextRender|SetText (Variables|Default|GetCharacter%20Info) (Utilities|Text|FormatText ""))
  (if (Variables|/Game/Blueprints/PuzzleBlockGrid.PuzzleBlockGrid_C|Gethuman (Variables|Default|Getowning%20grid))
    (Rendering|Components|TextRender|SetText _funds (Utilities|Text|FormatText "Available Funds: {Available Funds}" (Variables|Default|GetAvailable%20Funds)))
    (Rendering|Components|TextRender|SetTextRenderColor _funds (Math|Color|MakeColor 255 255 255 100))
    (else
      (Rendering|Components|TextRender|SetText _funds (Utilities|Text|FormatText "")))))